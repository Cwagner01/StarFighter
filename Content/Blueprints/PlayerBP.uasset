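; Player-controlled ship Blueprint that routes move, pitch, yaw, roll and fire input to the matching movement and weapon functions.
; On BeginPlay it initializes at the world origin, negates ForwardVector and rotates the ship mesh by the inverse of DefaultRot.
; InitializePlayer receives the PilotController's ship but does not use it.
; Tick accumulates time since the last shot, limiting presses of Fire to FireRate shots per second.
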(event EventBeginPlay
  (|CallParentFunction)
  (CallFunction|InitializePlayer "0, 0, 0" (Variables|/Game/Blueprints/Pilot_ControllerBP.Pilot_ControllerBP_C|Getship (Variables|Default|GetpilotController))))

(event Collision|EventActorBeginOverlap
  (params (OtherActor :type Actor%20Object%20Reference)))

(event EventTick
  (params (DeltaSeconds :type Float%20%28single-precision%29))
  (bind _output_get (Variables|Default|SettimeSinceTick DeltaSeconds))
  (Variables|Default|SettimeSinceLastShot (+ (Variables|Default|GettimeSinceLastShot) _output_get)))

(event Input|ActionEvents|InputActionFire
  (params (Key :type Key%20Structure :default "AnyKey"))
  (:Pressed
    (if (>= (Variables|Default|GettimeSinceLastShot) (/ 1.0 (Variables|Default|GetfireRate)))
      (Variables|Default|SettimeSinceLastShot 0.0)
      (CallFunction|Fire))))

(event Input|AxisEvents|InputAxisMove
  (params (AxisValue :type Float%20%28single-precision%29))
  (CallFunction|Move AxisValue))

(event Input|AxisEvents|InputAxisRoll
  (params (AxisValue :type Float%20%28single-precision%29))
  (CallFunction|Roll AxisValue))

(event Input|AxisEvents|InputAxisPitch
  (params (AxisValue :type Float%20%28single-precision%29))
  (CallFunction|Pitch AxisValue))

(event Input|AxisEvents|InputAxisYaw
  (params (AxisValue :type Float%20%28single-precision%29))
  (CallFunction|Yaw AxisValue))

(fn ConstructionScript)

(fn InitializePlayer
  (params (spawnLoc :type Vector) (ship :type Ship%20Struct%20Structure))
  (CallFunction|Initialize spawnLoc)
  (Variables|Default|SetforwardVector (* (Variables|Default|GetforwardVector) -1.0))
  (Transformation|AddRelativeRotation (Variables|Default|GetshipMesh) (Class|KismetMathLibrary|NegateRotator (Variables|Default|GetdefaultRot)) false false))