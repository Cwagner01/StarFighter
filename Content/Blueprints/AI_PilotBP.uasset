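; AI pilot that flies a ship, patrolling around its spawn and dogfighting hostile pilots.
; A Tick-driven state machine cycles random goals through eight octant volumes in PATROL, or matches target speed and fires in ENGAGE, leading shots by solving a quadratic intercept.
; Sighted pilots become targets through a distance and skill roll, filtered by faction and existing attackers.
; Death lowers the killer's faction standing, plays an explosion and decrements the spawner count.
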(event OnSeePawn(PawnSensing)
  (params (Pawn :type Pawn%20Object%20Reference))
  (bind _aspilot_bp (Utilities|Casting|CastToPilotBP Pawn))
  (if (not (== (Variables|Default|Gettarget) _aspilot_bp)) ; New target == curr target?
    (if (not (Variables|/Game/Blueprints/PilotBP.PilotBP_C|GetisDisabled _aspilot_bp))
      (CallFunction|Detect _aspilot_bp))))

(event Game|Damage|EventAnyDamage
  (params (Damage :type Float%20%28single-precision%29) (DamageType :type Damage%20Type%20Object%20Reference) (InstigatedBy :type Controller%20Object%20Reference) (DamageCauser :type Actor%20Object%20Reference))
  (if (not (Variables|Default|GetisDisabled))
    (bind _aspilot_bp (Utilities|Casting|CastToPilotBP DamageCauser))
    (CallFunction|TakeDamageAI Damage _aspilot_bp)))

(event Collision|EventActorBeginOverlap
  (params (OtherActor :type Actor%20Object%20Reference)))

(event EventBeginPlay
  (|CallParentFunction))

(event EventTick
  (params (DeltaSeconds :type Float%20%28single-precision%29))
  (|CallParentFunction DeltaSeconds)
  (if (not (Variables|Default|GetisDisabled))
    (switch Utilities|FlowControl|Switch|SwitchonAIStateEnum (Variables|Default|GetaiStateEnum)
      (:NewEnumerator2
        (CallFunction|Patrol))
      (:NewEnumerator3
        (if (Variables|/Game/Blueprints/PilotBP.PilotBP_C|GetisDisabled (Variables|Default|Gettarget))
          (Variables|Default|SetcurrTargetActive false)
          (Variables|Default|SetaiStateEnum "NewEnumerator2")
          (else
            (CallFunction|Engage)))))))

(fn ConstructionScript
  (|CallParentFunction))

(fn GeneratePatrolVolumes
  (bind _patrolradius (Variables|Default|GetpatrolRadius))
  (bind _patrolvolumes (Variables|Default|GetpatrolVolumes))
  (bind _spawnlocation (Variables|Default|GetspawnLocation))
  (bind (_x _y _z) (Math|Vector|BreakVector _spawnlocation))
  (Utilities|Array|Add _patrolvolumes (Utilities|Struct|MakeCubeVolume _x (+ _x _patrolradius) (- _y _patrolradius) _y _z (+ _z _patrolradius)))
  (Utilities|Array|Add _patrolvolumes (Utilities|Struct|MakeCubeVolume (- _x _patrolradius) _x (- _y _patrolradius) _y _z (+ _z _patrolradius)))
  (Utilities|Array|Add _patrolvolumes (Utilities|Struct|MakeCubeVolume (- _x _patrolradius) _x _y (+ _y _patrolradius) _z (+ _z _patrolradius)))
  (Utilities|Array|Add _patrolvolumes (Utilities|Struct|MakeCubeVolume _x (+ _x _patrolradius) _y (+ _y _patrolradius) _z (+ _z _patrolradius)))
  (Utilities|Array|Add _patrolvolumes (Utilities|Struct|MakeCubeVolume _x (+ _x _patrolradius) (- _y _patrolradius) _y (- _z _patrolradius) _z))
  (Utilities|Array|Add _patrolvolumes (Utilities|Struct|MakeCubeVolume (- _x _patrolradius) _x (- _y _patrolradius) _y (- _z _patrolradius) _z))
  (Utilities|Array|Add _patrolvolumes (Utilities|Struct|MakeCubeVolume (- _x _patrolradius) _x _y (+ _y _patrolradius) (- _z _patrolradius) _z))
  (Utilities|Array|Add _patrolvolumes (Utilities|Struct|MakeCubeVolume _x (+ _x _patrolradius) _y (+ _y _patrolradius) (- _z _patrolradius) _z)))

(fn DeterminePatrolVolume
  (bind _currlocation (Variables|Default|GetcurrLocation))
  (bind (_x _y _z) (Math|Vector|BreakVector _currlocation))
  (for (_array_element _array_index) (Variables|Default|GetpatrolVolumes)
    (if (Math|Boolean|ANDBoolean (>= _x (.minX (Utilities|Struct|BreakCubeVolume _array_element))) (<= _x (.maxX (Utilities|Struct|BreakCubeVolume _array_element))) (>= _y (.minY (Utilities|Struct|BreakCubeVolume _array_element))) (<= _y (.maxY (Utilities|Struct|BreakCubeVolume _array_element))) (>= _z (.minZ (Utilities|Struct|BreakCubeVolume _array_element))) (<= _z (.maxZ (Utilities|Struct|BreakCubeVolume _array_element))))
      (return _array_index)))
  (return -1))

(fn Patrol
  (bind _distthreshold (LocalVariables|GetdistThreshold))
  (bind _distance (CallFunction|Distanceto (Variables|Default|GetcurrLocation) (Variables|Default|GetgoalLocation)))
  (bind _output_get (Variables|Default|SettimeSinceDistCheck (+ (Variables|Default|GettimeSinceTick) (Variables|Default|GettimeSinceDistCheck))))
  (Variables|Default|SetlastDistVal _distance)
  (if (<= _distance 15.0)
    (CallFunction|GetNextGoalLocation :!label _label)
    (else
      ;[1 1 1] Break out of look-at lock
      (if (>= _output_get 1.0)
        (Variables|Default|SettimeSinceDistCheck 0.0)
        (if (and (<= _distance (+ (Variables|Default|GetlastDistVal) _distthreshold)) (>= _distance (- (Variables|Default|GetlastDistVal) _distthreshold)))
          (bind _output_get_2 (Variables|Default|SetdistCount (+ (Variables|Default|GetdistCount) 1)))
          (if (>= _output_get_2 5)
            (Variables|Default|SetdistCount 0)
            (goto _label)
            (else
              _))))))
  (CallFunction|MoveToward 1))

(fn Idle)

(fn Engage
  (if (Variables|Default|GetcurrTargetActive)
    (bind _output_get (Variables|Default|SetgoalLocation (Transformation|GetActorLocation (Variables|Default|Gettarget))))
    ;[1 1 1] Determine movement action
    (bind _distance (CallFunction|Distanceto (Variables|Default|GetcurrLocation) _output_get))
    (if (<= _distance (Variables|Default|GetmaxRange))
      (if (>= _distance (Variables|Default|GetminRange))
        (CallFunction|MoveToward) ; Match speed
        (else
          (CallFunction|MoveToward -1) ; Decelerate
        ))
      (CallFunction|Aim)
      (Variables|Default|SetshouldFire true)
      (CallFunction|HandleWeaponFiring)
      (else
        (CallFunction|MoveToward 1) ; Accelerate
        (Variables|Default|SetshouldFire false)
        (Variables|Default|SetgoalLocation (Transformation|GetActorLocation (Variables|Default|Gettarget)))))
    (else
      (Variables|Default|SetaiStateEnum "NewEnumerator2"))))

(fn GetNextGoalLocation
  (bind _patrolvolumes (Variables|Default|GetpatrolVolumes))
  (switch Utilities|FlowControl|Switch|SwitchonAIStateEnum (Variables|Default|GetaiStateEnum)
    (:NewEnumerator2
      ;[1 1 1] Patrol
      ;;[1 1 1] Determine which patrol volume to move to next
      (bind _currvolume (CallFunction|DeterminePatrolVolume))
      (if (== _currvolume -1)
        ;;[1 1 1] Get new goal location
        (bind _goalloc (CallFunction|GenerateCubeLocation (Utilities|Array|Get(acopy) _patrolvolumes) :!label _label))
        (Variables|Default|SetgoalLocation _goalloc)
        (elif (>= (+ _currvolume 1) (Utilities|Array|Length _patrolvolumes))
          (goto _label)
          (else
            (bind _goalloc_2 (CallFunction|GenerateCubeLocation (Utilities|Array|Get(acopy) _patrolvolumes (+ _currvolume 1))))
            (Variables|Default|SetgoalLocation _goalloc_2)))))))

(fn GenerateCubeLocation
  (params (patrolCube :type Cube%20Volume%20Structure))
  (bind (_minx _maxx _miny _maxy _minz _maxz) (Utilities|Struct|BreakCubeVolume patrolCube))
  (return (Math|Vector|MakeVector (+ (* (/ (Math|Conversions|ToFloat(Integer) (Math|Random|RandomIntegerinRange 0 100)) 1e+02) (- _maxx _minx)) _minx) (+ (* (/ (Math|Conversions|ToFloat(Integer) (Math|Random|RandomIntegerinRange 0 100)) 1e+02) (- _maxy _miny)) _miny) (+ (* (/ (Math|Conversions|ToFloat(Integer) (Math|Random|RandomIntegerinRange 0 100)) 1e+02) (- _maxz _minz)) _minz))))

(fn TurntoFaceArb
  (bind _output_get (LocalVariables|SettmpForward (Variables|Default|GetforwardVector)))
  (bind _output_get_2 (LocalVariables|SettmpUp (Variables|Default|GetupVector)))
  (bind _output_get_3 (LocalVariables|SetgoalDir (Math|Vector|RotateVector (Math|Vector|Normalize (- (Variables|Default|GetgoalLocation) (Variables|Default|GetcurrLocation))) (Class|KismetMathLibrary|NegateRotator (Math|Rotator|MakeRotationfromAxes _output_get (Math|Vector|CrossProduct _output_get_2 _output_get) _output_get_2)))))
  (Transformation|AddActorLocalRotation (Math|Vector|RotatorfromAxisandAngle (Math|Vector|CrossProduct "1.000000, 0, 0" _output_get_3) (* (* (Variables|Default|GetturnRate) (Variables|Default|GettimeSinceTick)) (Class|KismetMathLibrary|DegAcos (Math|Vector|DotProduct _output_get_3 "1.000000, 0, 0")))) false false)
  (Variables|Default|SetforwardVector (Transformation|GetActorForwardVector))
  (Variables|Default|SetupVector (Transformation|GetActorUpVector))
  (return (Class|KismetMathLibrary|DegAcos (Math|Vector|DotProduct _output_get_3 "1.000000, 0, 0"))))

(fn Evade)

(fn Detect
  (params (newTarget :type Pilot%20BP%20Object%20Reference))
  (bind _returnvalue (Transformation|GetActorLocation newTarget))
  (bind _currlocation (Variables|Default|GetcurrLocation))
  (bind _targetedby (Variables|/Game/Blueprints/PilotBP.PilotBP_C|GettargetedBy newTarget))
  (bind (_x _y _z) (Math|Vector|BreakVector _returnvalue))
  (bind (_x_2 _y_2 _z_2) (Math|Vector|BreakVector _currlocation))
  (bind _returnvalue_2 (- _x _x_2))
  (bind _returnvalue_3 (- _y _y_2))
  (bind _returnvalue_4 (- _z _z_2))
  (bind _returnvalue_5 (Math|Float|Square _returnvalue_2))
  (bind _returnvalue_6 (Math|Float|Square _returnvalue_3))
  (bind _returnvalue_7 (Math|Float|Square _returnvalue_4))
  (bind _returnvalue_8 (+ _returnvalue_5 _returnvalue_6 _returnvalue_7))
  (bind _returnvalue_9 (Math|Float|Sqrt _returnvalue_8))
  (bind _output_get (LocalVariables|SetmaxDistance 7.5e+03))
  ;[1 1 1] Determine detection chance
  (if (<= _returnvalue_9 _output_get)
    ;[1 1 1] Determine detection
    (if (<= (Math|Conversions|ToFloat(Integer) (Math|Random|RandomIntegerinRange 1 100)) (+ 4e+01 (* (Variables|Default|Getskill) (* (- 1.0 (/ _returnvalue_9 _output_get)) 5e+01))))
      ;[1 1 1] Set new target
      (if (not (Variables|Default|GetcurrTargetActive))
        (bind _factionval (Default|GetFactionVal newTarget (Variables|Default|Getfaction)))
        (if (not (>= _factionval 0.0))
          (if (== _targetedby 0)
            (Default|Targeted newTarget self :!label _label)
            (Variables|Default|Settarget newTarget)
            (Variables|Default|SetcurrTargetActive true)
            (Variables|Default|SetaiStateEnum "NewEnumerator3")
            (elif (Variables|/Game/Blueprints/PilotBP.PilotBP_C|GetisDisabled _targetedby)
              (goto _label))))))))

(fn MoveToward
  (params (rangeIndicator :type Integer))
  (bind _returnvalue (Math|Conversions|ToFloat(Integer) rangeIndicator))
  (bind _target (Variables|Default|Gettarget))
  (bind _currspeed (Variables|Default|GetcurrSpeed))
  (bind _currspeed_2 (Variables|/Game/Blueprints/PilotBP.PilotBP_C|GetcurrSpeed _target))
  (bind _degrees (CallFunction|TurntoFaceArb))
  (if (>= _degrees 6e+01)
    (CallFunction|Accelerate -1.0)
    (elif (!= _returnvalue 0.0)
      (CallFunction|Accelerate _returnvalue :!label _label)
      (elif (!= _target 0)
        (if (> _currspeed_2 _currspeed)
          (CallFunction|Accelerate 1.0)
          (elif (< _currspeed_2 _currspeed)
            (CallFunction|Accelerate -1.0)
            (else
              (CallFunction|Accelerate 0.0))))
        (else
          (goto _label)))))
  (Transformation|SetActorLocation (+ (Variables|Default|GetcurrLocation) (* (Variables|Default|GetforwardVector) (* (Variables|Default|GetcurrSpeed) (Variables|Default|GettimeSinceTick)))) false false)
  (Variables|Default|SetcurrLocation (+ (Variables|Default|GetcurrLocation) (* (Variables|Default|GetforwardVector) (* (Variables|Default|GetcurrSpeed) (Variables|Default|GettimeSinceTick))))))

(fn InitializeAI
  (params (spawnLoc :type Vector) (ship :type Ship%20Struct%20Structure) (skill :type Float%20%28single-precision%29))
  (CallFunction|Initialize spawnLoc ship)
  (Variables|Default|Setskill skill)
  (Variables|Default|SetaiStateEnum "NewEnumerator2")
  (CallFunction|GeneratePatrolVolumes)
  (CallFunction|GetNextGoalLocation))

(fn Aim
  (bind _currlocation (Variables|Default|GetcurrLocation))
  (bind _target (Variables|Default|Gettarget))
  (bind _returnvalue (Transformation|GetActorLocation _target))
  (bind _returnvalue_2 (Transformation|GetActorForwardVector _target))
  (bind _currspeed (Variables|/Game/Blueprints/PilotBP.PilotBP_C|GetcurrSpeed _target))
  (bind _returnvalue_3 (- _returnvalue _currlocation))
  (bind _returnvalue_4 (* _returnvalue_2 _currspeed))
  (bind _returnvalue_5 (Math|Vector|DotProduct _returnvalue_4 _returnvalue_3))
  (bind _returnvalue_6 (* 2 _returnvalue_5))
  (bind _weapon (CallFunction|GetSingleWeapon (Variables|/Game/Blueprints/Pilot_ControllerBP.Pilot_ControllerBP_C|Getship (Variables|Default|GetpilotController))))
  (if (and (> (- (/ (* -1 _returnvalue_6) (* 2 (- (Math|Vector|DotProduct _returnvalue_4 _returnvalue_4) (Math|Float|Square (.laserSpeed (Utilities|Struct|BreakWeaponStruct _weapon)))))) (/ (Math|Float|Sqrt (- (Math|Float|Square _returnvalue_6) (* (Math|Vector|DotProduct _returnvalue_3 _returnvalue_3) (- (Math|Vector|DotProduct _returnvalue_4 _returnvalue_4) (Math|Float|Square (.laserSpeed (Utilities|Struct|BreakWeaponStruct _weapon)))) 4.0))) (* 2 (- (Math|Vector|DotProduct _returnvalue_4 _returnvalue_4) (Math|Float|Square (.laserSpeed (Utilities|Struct|BreakWeaponStruct _weapon))))))) (+ (/ (* -1 _returnvalue_6) (* 2 (- (Math|Vector|DotProduct _returnvalue_4 _returnvalue_4) (Math|Float|Square (.laserSpeed (Utilities|Struct|BreakWeaponStruct _weapon)))))) (/ (Math|Float|Sqrt (- (Math|Float|Square _returnvalue_6) (* (Math|Vector|DotProduct _returnvalue_3 _returnvalue_3) (- (Math|Vector|DotProduct _returnvalue_4 _returnvalue_4) (Math|Float|Square (.laserSpeed (Utilities|Struct|BreakWeaponStruct _weapon)))) 4.0))) (* 2 (- (Math|Vector|DotProduct _returnvalue_4 _returnvalue_4) (Math|Float|Square (.laserSpeed (Utilities|Struct|BreakWeaponStruct _weapon)))))))) (> (+ (/ (* -1 _returnvalue_6) (* 2 (- (Math|Vector|DotProduct _returnvalue_4 _returnvalue_4) (Math|Float|Square (.laserSpeed (Utilities|Struct|BreakWeaponStruct _weapon)))))) (/ (Math|Float|Sqrt (- (Math|Float|Square _returnvalue_6) (* (Math|Vector|DotProduct _returnvalue_3 _returnvalue_3) (- (Math|Vector|DotProduct _returnvalue_4 _returnvalue_4) (Math|Float|Square (.laserSpeed (Utilities|Struct|BreakWeaponStruct _weapon)))) 4.0))) (* 2 (- (Math|Vector|DotProduct _returnvalue_4 _returnvalue_4) (Math|Float|Square (.laserSpeed (Utilities|Struct|BreakWeaponStruct _weapon))))))) 0.0))
    (Variables|Default|SetgoalLocation (+ _returnvalue (* _returnvalue_4 (+ (/ (* -1 _returnvalue_6) (* 2 (- (Math|Vector|DotProduct _returnvalue_4 _returnvalue_4) (Math|Float|Square (.laserSpeed (Utilities|Struct|BreakWeaponStruct _weapon)))))) (/ (Math|Float|Sqrt (- (Math|Float|Square _returnvalue_6) (* (Math|Vector|DotProduct _returnvalue_3 _returnvalue_3) (- (Math|Vector|DotProduct _returnvalue_4 _returnvalue_4) (Math|Float|Square (.laserSpeed (Utilities|Struct|BreakWeaponStruct _weapon)))) 4.0))) (* 2 (- (Math|Vector|DotProduct _returnvalue_4 _returnvalue_4) (Math|Float|Square (.laserSpeed (Utilities|Struct|BreakWeaponStruct _weapon))))))))))
    (else
      (Variables|Default|SetgoalLocation (+ _returnvalue (* _returnvalue_4 (- (/ (* -1 _returnvalue_6) (* 2 (- (Math|Vector|DotProduct _returnvalue_4 _returnvalue_4) (Math|Float|Square (.laserSpeed (Utilities|Struct|BreakWeaponStruct _weapon)))))) (/ (Math|Float|Sqrt (- (Math|Float|Square _returnvalue_6) (* (Math|Vector|DotProduct _returnvalue_3 _returnvalue_3) (- (Math|Vector|DotProduct _returnvalue_4 _returnvalue_4) (Math|Float|Square (.laserSpeed (Utilities|Struct|BreakWeaponStruct _weapon)))) 4.0))) (* 2 (- (Math|Vector|DotProduct _returnvalue_4 _returnvalue_4) (Math|Float|Square (.laserSpeed (Utilities|Struct|BreakWeaponStruct _weapon)))))))))))))

(fn TakeDamageAI
  (params (damage :type Float%20%28single-precision%29) (damager :type Pilot%20BP%20Object%20Reference))
  (bind _targetedby (Variables|Default|GettargetedBy))
  (bind _parentspawner (Variables|Default|GetparentSpawner))
  (CallFunction|TakeDamage damage)
  (if (== (Variables|Default|Gethealth) 0.0)
    (Default|ChangeFactionVal damager (Variables|Default|Getfaction) -1.0)
    (Components|StaticMesh|SetStaticMesh (Variables|Default|GetshipMesh) 0)
    (Variables|Default|SetisDisabled true)
    (Audio|Components|Audio|Play (Variables|Default|GetExplosionAudio) 0.0)
    (Components|Activation|ToggleActive (Variables|Default|GetExplosionParticles))
    (bind _result (Math|Integer|DecrementInt (Variables|/Game/Blueprints/AI_Spawner_BP.AI_Spawner_BP_C|GetnumSpawns _parentspawner))
      (:%20%20
        (Variables|/Game/Blueprints/AI_Spawner_BP.AI_Spawner_BP_C|SetnumSpawns _parentspawner _result)
        (if (not (== _targetedby 0))
          (bind _asai_pilot_bp (Utilities|Casting|CastToAI_PilotBP _targetedby))
          (Variables|AI_PilotBP_C|SetcurrTargetActive _asai_pilot_bp false)
          (Variables|AI_PilotBP_C|Settarget _asai_pilot_bp 0))))))