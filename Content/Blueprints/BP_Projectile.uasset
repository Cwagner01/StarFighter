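; BP_Projectile is a tinted projectile actor that flies in a straight line at a set speed.
; On BeginPlay it colours its dynamic material, then LookAt rotates it by axis-angle using the incoming ForwardVector and stores the resulting forward direction.
; Tick advances a tracked CurrLoc along that direction without sweeping.
; The overlap event is empty; the owner-filtered damage and destroy logic is disconnected and never runs.
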(event OnComponentBeginOverlap(Projectile)
  (params (OverlappedComponent :type Primitive%20Component%20Object%20Reference) (OtherActor :type Actor%20Object%20Reference) (OtherComp :type Primitive%20Component%20Object%20Reference) (OtherBodyIndex :type Integer) (bFromSweep :type Boolean) (SweepResult :type Hit%20Result%20Structure%20%28by%20ref%29)))

(event EventBeginPlay
  (Rendering|Material|SetVectorParameterValue (Variables|Default|GetprojectileMaterial) "Color2" (Variables|Default|GetprojectileColor) :!class /Script/Engine.MaterialInstanceDynamic)
  (CallFunction|Lookat))

(event EventTick
  (params (DeltaSeconds :type Float%20%28single-precision%29))
  (CallFunction|Move DeltaSeconds))

(fn ConstructionScript
  (Transformation|SetActorScale3D "1.000000,0.600000,0.600000")
  (bind _returnvalue (Rendering|Material|CreateDynamicMaterialInstance (Variables|Default|GetProjectile) 0 "/Game/Particles/Projectile.Projectile" :!class /Script/Engine.PrimitiveComponent))
  (Variables|Default|SetprojectileMaterial _returnvalue))

(fn Lookat
  (bind _output_get (LocalVariables|SettmpForward (Transformation|GetActorForwardVector)))
  (bind _output_get_2 (LocalVariables|SettmpUp (Transformation|GetActorUpVector)))
  (bind _output_get_3 (LocalVariables|SetgoalDir (Math|Vector|RotateVector (Math|Vector|Normalize (- (Variables|Default|GetforwardVector) _output_get)) (Class|KismetMathLibrary|NegateRotator (Math|Rotator|MakeRotationfromAxes _output_get (Math|Vector|CrossProduct _output_get_2 _output_get) _output_get_2)))))
  (Transformation|AddActorLocalRotation (Math|Vector|RotatorfromAxisandAngle (Math|Vector|CrossProduct "1.000000, 0, 0" _output_get_3) (Class|KismetMathLibrary|DegAcos (Math|Vector|DotProduct _output_get_3 "1.000000, 0, 0"))) false false)
  (Variables|Default|SetforwardVector (Transformation|GetActorForwardVector)))

(fn Move
  (params (deltaTime :type Float%20%28single-precision%29))
  (Transformation|SetActorLocation (+ (Variables|Default|GetcurrLoc) (* (Variables|Default|GetforwardVector) (* deltaTime (Variables|Default|Getspeed)))) false false)
  (Variables|Default|SetcurrLoc (+ (Variables|Default|GetcurrLoc) (* (Variables|Default|GetforwardVector) (* deltaTime (Variables|Default|Getspeed))))))