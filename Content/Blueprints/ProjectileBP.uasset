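; Projectile actor that flies in a straight line and damages AI pilots it overlaps.
; The construction script scales it, creates a dynamic material and places it at its starting location; BeginPlay applies the projectile color.
; Tick moves it manually along its forward vector without sweeping, destroying it once accumulated distance reaches the maximum.
; Overlaps ignore itself and its owner, and only an exact AI_PilotBP class match takes damage and destroys the projectile.
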(event OnComponentBeginOverlap(Projectile)
  (params (OverlappedComponent :type Primitive%20Component%20Object%20Reference) (OtherActor :type Actor%20Object%20Reference) (OtherComp :type Primitive%20Component%20Object%20Reference) (OtherBodyIndex :type Integer) (bFromSweep :type Boolean) (SweepResult :type Hit%20Result%20Structure%20%28by%20ref%29))
  (if (and (!= (Variables|Default|GetprojectileOwner) OtherActor) (!= OtherActor self))
    (if (== (Utilities|GetClass OtherActor) "/Game/Blueprints/AI_PilotBP.AI_PilotBP_C")
      (Game|Damage|ApplyDamage OtherActor (Variables|Default|Getdamage) 0 0)
      (Actor|DestroyActor))))

(event EventBeginPlay
  (Rendering|Material|SetVectorParameterValue (Variables|Default|GetprojectileMaterial) "Color2" (Variables|Default|GetprojectileColor) :!class /Script/Engine.MaterialInstanceDynamic))

(event EventTick
  (params (DeltaSeconds :type Float%20%28single-precision%29))
  (CallFunction|Move DeltaSeconds)
  (if (>= (Variables|Default|GetcurrDist) (Variables|Default|GetmaxDist))
    (Actor|DestroyActor)))

(fn ConstructionScript
  (Transformation|SetActorScale3D "1.000000,0.700000,0.700000")
  (bind _returnvalue (Rendering|Material|CreateDynamicMaterialInstance (Variables|Default|GetProjectile) 0 "/Game/Particles/Projectile.Projectile" :!class /Script/Engine.PrimitiveComponent))
  (Variables|Default|SetprojectileMaterial _returnvalue)
  (Transformation|SetActorLocation (Variables|Default|GetcurrLoc) false false))

(fn Move
  (params (deltaTime :type Float%20%28single-precision%29))
  (Transformation|SetActorLocation (+ (Variables|Default|GetcurrLoc) (* (Variables|Default|GetforwardVector) (* deltaTime (Variables|Default|Getspeed)))) false false)
  (bind _distance (CallFunction|Distanceto (Variables|Default|GetcurrLoc) (+ (Variables|Default|GetcurrLoc) (* (Variables|Default|GetforwardVector) (* deltaTime (Variables|Default|Getspeed))))))
  (Variables|Default|SetcurrDist (+ (Variables|Default|GetcurrDist) _distance))
  (Variables|Default|SetcurrLoc (+ (Variables|Default|GetcurrLoc) (* (Variables|Default|GetforwardVector) (* deltaTime (Variables|Default|Getspeed))))))