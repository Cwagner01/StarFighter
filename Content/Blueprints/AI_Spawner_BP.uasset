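; AI spawner actor that creates AI_PilotBP pawns at its own location until a maximum spawn count is reached.
; Tick advances timers and asks DetermineSpawn, which rolls periodically within a min-max time window, with odds rising linearly until a spawn is guaranteed.
; Spawn initializes each pilot with its location, its AI controller's ship and a fixed skill, then records it.
; The count only increases, so the cap is a lifetime total.
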(event EventBeginPlay)

(event Collision|EventActorBeginOverlap
  (params (OtherActor :type Actor%20Object%20Reference)))

(event EventTick
  (params (DeltaSeconds :type Float%20%28single-precision%29))
  (Variables|Default|SettimeSinceSpawn (+ DeltaSeconds (Variables|Default|GettimeSinceSpawn)))
  (Variables|Default|SettimeSinceTry (+ DeltaSeconds (Variables|Default|GettimeSinceTry)))
  (if (< (Variables|Default|GetnumSpawns) (Variables|Default|GetmaxSpawns))
    (bind _shouldspawn (CallFunction|DetermineSpawn))
    (if _shouldspawn
      (CallFunction|Spawn))))

(fn ConstructionScript)

(fn Spawn
  (bind _returnvalue (Transformation|GetActorLocation))
  (bind _returnvalue_2 (Game|SpawnActorfromClass "/Game/Blueprints/AI_PilotBP.AI_PilotBP_C" (Math|Conversions|ToTransform(Vector) _returnvalue) "AlwaysSpawn" 0 0))
  (bind _asai_controller_bp (Utilities|Casting|CastToAI_ControllerBP (Pawn|GetController _returnvalue_2)))
  (Default|InitializeAI _returnvalue_2 _returnvalue (Variables|/Game/Blueprints/Pilot_ControllerBP.Pilot_ControllerBP_C|Getship _asai_controller_bp) 1.0)
  (Utilities|Array|Add (Variables|Default|Getspawns) _returnvalue_2)
  (Variables|Default|SettimeSinceSpawn 0.0)
  (Variables|Default|SetnumSpawns (+ (Variables|Default|GetnumSpawns) 1)))

(fn DetermineSpawn
  (bind _maxtimeuntilspawn (Variables|Default|GetmaxTimeUntilSpawn))
  (bind _timesincespawn (Variables|Default|GettimeSinceSpawn))
  (bind _mintimeuntilspawn (Variables|Default|GetminTimeUntilSpawn))
  (if (< (Variables|Default|GetnumSpawns) (Variables|Default|GetmaxSpawns)) ; numSpawns < maxSpawns
    (if (>= _timesincespawn _maxtimeuntilspawn) ; time >= maxTime
      (return true) ; Return true
      (elif (>= _timesincespawn _mintimeuntilspawn) ; time >= minTime
        (if (>= (Variables|Default|GettimeSinceTry) (Variables|Default|GetmaxTimeBeforeTry)) ; time to try?
          (if (<= (Math|Random|RandomIntegerinRange 1 100) (Math|Float|Truncate (* (/ (- _timesincespawn _mintimeuntilspawn) (- _maxtimeuntilspawn _mintimeuntilspawn)) 1e+02))) ; Time weighted chance to spawn
            (Variables|Default|SettimeSinceTry 0.0)
            (return true) ; Return true
            (else
              (Variables|Default|SettimeSinceTry 0.0)))))))
  (return false) ; Return false
)