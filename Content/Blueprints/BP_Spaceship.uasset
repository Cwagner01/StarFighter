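; BP_Spaceship is an input-driven ship with six-axis-style flight controls, twin weapons and health.
; Yaw, pitch and roll apply local rotation while manually rotating stored Forward and Up vectors, and Move does a swept location change along Forward.
; Holding Fire spawns BP_Projectile from Left and Right immediately, then repeats on a looping timer until release.
; AnyDamage reduces clamped Health and destroys the ship at zero.
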(event Custom|FireReset
  ;[1 1 1] Fire Weapons
  (CallFunction|Fire (Variables|Default|GetLeft))
  (CallFunction|Fire (Variables|Default|GetRight)))

(event Game|Damage|EventAnyDamage
  (params (Damage :type Float%20%28single-precision%29) (DamageType :type Damage%20Type%20Object%20Reference) (InstigatedBy :type Controller%20Object%20Reference) (DamageCauser :type Actor%20Object%20Reference))
  (CallFunction|TakeDamage Damage))

(event Input|ActionEvents|InputActionFire
  (params (Key :type Key%20Structure :default "AnyKey"))
  ;[1 1 1] Fire Weapons
  (:Pressed
    (bind _returnvalue (Utilities|Time|SetTimerbyFunctionName 0 "FireReset" 2.0 true))
    (Variables|Default|SetTimeHandle _returnvalue)
    (CallFunction|Fire (Variables|Default|GetLeft))
    (CallFunction|Fire (Variables|Default|GetRight)))
  (:Released
    (Utilities|Time|ClearandInvalidateTimerbyHandle (Variables|Default|GetTimeHandle))))

(event Input|AxisEvents|InputAxisYaw
  (params (AxisValue :type Float%20%28single-precision%29))
  ;[1 1 1] Movement
  (Transformation|AddActorLocalRotation (Math|Rotator|MakeRotator 0.0 0.0 AxisValue) false false)
  (bind _output_get (Variables|Default|SetForward_Vector (Math|Vector|RotateVectorAroundAxis (Variables|Default|GetForward_Vector) AxisValue (Variables|Default|GetUp_Vector)))))

(event Input|AxisEvents|InputAxisPitch
  (params (AxisValue :type Float%20%28single-precision%29))
  ;[1 1 1] Movement
  (Transformation|AddActorLocalRotation (Math|Rotator|MakeRotator 0.0 AxisValue 0.0) false false)
  (bind _output_get (Variables|Default|SetForward_Vector (Math|Vector|RotateVectorAroundAxis (Variables|Default|GetForward_Vector) AxisValue (Math|Vector|CrossProduct (Variables|Default|GetUp_Vector) (Variables|Default|GetForward_Vector)))))
  (bind _output_get_2 (Variables|Default|SetUp_Vector (Math|Vector|RotateVectorAroundAxis (Variables|Default|GetUp_Vector) AxisValue (Math|Vector|CrossProduct (Variables|Default|GetUp_Vector) (Variables|Default|GetForward_Vector))))))

(event Input|AxisEvents|InputAxisRoll
  (params (AxisValue :type Float%20%28single-precision%29))
  ;[1 1 1] Movement
  (Transformation|AddActorLocalRotation (Math|Rotator|MakeRotator AxisValue 0.0 0.0) false false)
  (bind _output_get (Variables|Default|SetUp_Vector (Math|Vector|RotateVectorAroundAxis (Variables|Default|GetUp_Vector) AxisValue (Variables|Default|GetForward_Vector)))))

(event Input|AxisEvents|InputAxisMove
  (params (AxisValue :type Float%20%28single-precision%29))
  ;[1 1 1] Movement
  (Transformation|SetActorLocation (+ (Transformation|GetActorLocation) (* (Variables|Default|GetForward_Vector) (* 7.5 AxisValue))) true false))

(fn ConstructionScript)

(fn Fire
  (params (Location :type Scene%20Component%20Object%20Reference))
  (Game|SpawnActorfromClass "/Game/Blueprints/BP_Projectile.BP_Projectile_C" (Transformation|GetWorldTransform Location) "Undefined" 0 (Math|Color|MakeColor 0.0 0.315 0.023807 0.9) "-100.000000,0.000000,0.000000" self))

(fn TakeDamage
  (params (damage :type Float%20%28single-precision%29))
  (Variables|Default|SetHealth (Math|Float|Clamp(Float) (- (Variables|Default|GetHealth) damage) 0.0 1e+02))
  (if (<= (Variables|Default|GetHealth) 0.0)
    (Actor|DestroyActor)))