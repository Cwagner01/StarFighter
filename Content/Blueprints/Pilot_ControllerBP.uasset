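; Pilot controller Blueprint that assembles a pilot's ship data from enum-selected hull, engine, shield, power and weapon parts.
; LoadComponents resolves each part through loader calls defined outside these graphs and packs the results into the Ship struct.
; LoadWeapons appends weapons to the Ship's weapon array, capped by the hull's slot count and positioned at its relative mount locations.
; BeginPlay, Tick and the construction script are empty.
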(event EventBeginPlay)

(event EventTick
  (params (DeltaSeconds :type Float%20%28single-precision%29)))

(fn ConstructionScript)

(fn LoadWeapons
  (params (hull :type Hull%20Struct%20Structure))
  (bind (_hullenum _hullstrength _numweapons _relativeweaponlocations) (Utilities|Struct|BreakHullStruct hull))
  (bind _weaponenums (Variables|Default|GetweaponEnums))
  (bind _returnvalue (Utilities|Array|Length _weaponenums))
  (bind _weapons (CallFunction|GetWeapons (Variables|Default|Getship)))
  (if (>= _returnvalue _numweapons) ; More weapons than slots
    (for _index (range 0 (- _numweapons 1))
      (bind _weapon (CallFunction|LoadWeapon (Utilities|Array|Get(acopy) _weaponenums _index)))
      (Utilities|Array|Add _weapons (Utilities|Struct|MakeWeaponStruct (Utilities|Array|Get(acopy) _relativeweaponlocations _index) (.damage (Utilities|Struct|BreakWeaponStruct _weapon)) (.fireRate (Utilities|Struct|BreakWeaponStruct _weapon)) (.fireCost (Utilities|Struct|BreakWeaponStruct _weapon)) (.laserSpeed (Utilities|Struct|BreakWeaponStruct _weapon)) (.laserColor (Utilities|Struct|BreakWeaponStruct _weapon)) (.energyCost (Utilities|Struct|BreakWeaponStruct _weapon)) (.damageOffset (Utilities|Struct|BreakWeaponStruct _weapon)) (.fireRateOffset (Utilities|Struct|BreakWeaponStruct _weapon)))))
    (else
      (for _index_2 (range 0 (- _returnvalue 1))
        (bind _weapon_2 (CallFunction|LoadWeapon (Utilities|Array|Get(acopy) _weaponenums _index_2)))
        (Utilities|Array|Add _weapons (Utilities|Struct|MakeWeaponStruct (Utilities|Array|Get(acopy) _relativeweaponlocations _index_2) (.damage (Utilities|Struct|BreakWeaponStruct _weapon_2)) (.fireRate (Utilities|Struct|BreakWeaponStruct _weapon_2)) (.fireCost (Utilities|Struct|BreakWeaponStruct _weapon_2)) (.laserSpeed (Utilities|Struct|BreakWeaponStruct _weapon_2)) (.laserColor (Utilities|Struct|BreakWeaponStruct _weapon_2)) (.energyCost (Utilities|Struct|BreakWeaponStruct _weapon_2)) (.damageOffset (Utilities|Struct|BreakWeaponStruct _weapon_2)) (.fireRateOffset (Utilities|Struct|BreakWeaponStruct _weapon_2)))))))
  (return _weapons))

(fn LoadComponents
  (bind _hull (CallFunction|LoadHull (Variables|Default|GethullEnum)))
  (bind _engine (CallFunction|LoadEngine (Variables|Default|GetengineEnum)))
  (bind _shield (CallFunction|LoadShield (Variables|Default|GetshieldEnum)))
  (bind _power (CallFunction|LoadPower (Variables|Default|GetpowerEnum)))
  (bind _weapons (CallFunction|LoadWeapons _hull))
  (Variables|Default|Setship (Utilities|Struct|MakeShipStruct _hull _engine _shield _power _weapons)))