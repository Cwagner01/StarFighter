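; Player-flyable spaceship that takes one of several ship looks and flies with six-degree rotation and forward throttle.
; Initialize sets mesh, material, scale and mesh rotation from a ship enum, then places the actor at its spawn location.
; Move axis adjusts clamped speed and advances a tracked location without sweep, using delta time cached in Tick.
; Pitch, yaw and roll rotate the actor locally while manually rotating stored forward and up vectors.
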(event EventBeginPlay)

(event Collision|EventActorBeginOverlap
  (params (OtherActor :type Actor%20Object%20Reference)))

(event EventTick
  (params (DeltaSeconds :type Float%20%28single-precision%29))
  (Variables|Default|SettimeSinceTick DeltaSeconds))

(event Input|AxisEvents|InputAxisMove
  (params (AxisValue :type Float%20%28single-precision%29))
  (CallFunction|Move AxisValue))

(event Input|AxisEvents|InputAxisRoll
  (params (AxisValue :type Float%20%28single-precision%29))
  (CallFunction|Roll AxisValue))

(event Input|AxisEvents|InputAxisPitch
  (params (AxisValue :type Float%20%28single-precision%29))
  (CallFunction|Pitch AxisValue))

(event Input|AxisEvents|InputAxisYaw
  (params (AxisValue :type Float%20%28single-precision%29))
  (CallFunction|Yaw AxisValue))

(fn ConstructionScript)

(fn Initialize
  (params (shipEnum :type EShipsEnumBP%20Enum) (spawnLoc :type Vector))
  (bind _shipmesh (Variables|Default|GetshipMesh))
  (bind _output_get (Variables|Default|SetshipEnum shipEnum))
  (switch Utilities|FlowControl|Switch|SwitchonEShipsEnumBP _output_get
    (:NewEnumerator0
      (Components|StaticMesh|SetStaticMesh _shipmesh "/Game/Ships/TieFighter/TieFighter.TieFighter" :!label _label)
      (Variables|Default|SetdefaultRot "0,0.000000, 0")
      (Transformation|SetActorScale3D "2.000000,2.000000,2.000000")
      (Rendering|Material|SetMaterial _shipmesh 0 "/Game/Ships/TieFighter/BasicMat.BasicMat"))
    (:NewEnumerator1
      (goto _label))
    (:NewEnumerator2
      (Components|StaticMesh|SetStaticMesh _shipmesh "/Game/Ships/dark_fighter_6/dark_fighter_6.dark_fighter_6")
      (Variables|Default|SetdefaultRot "0,180.000000, 0")
      (Transformation|SetActorScale3D "2.000000,2.000000,2.000000")
      (Rendering|Material|SetMaterial _shipmesh 0 "/Game/Ships/dark_fighter_6/dark_fighter_7.dark_fighter_7"))
    (:NewEnumerator3
      (Components|StaticMesh|SetStaticMesh _shipmesh "/Game/Ships/space_frigate_6/space_frigate_6.space_frigate_6")
      (Variables|Default|SetdefaultRot "0,180.000000,0.000000")
      (Transformation|SetActorScale3D "2.500000,2.500000,2.500000")
      (Rendering|Material|SetMaterial _shipmesh 0 "/Game/Ships/space_frigate_6/space_frigate_7.space_frigate_7"))
    (:NewEnumerator4
      (Components|StaticMesh|SetStaticMesh _shipmesh "/Game/Ships/SciFi_Fighter-MK6-OBJ/MK6_OBJ.MK6_OBJ")
      (Variables|Default|SetdefaultRot "0,-90.000000,90.000000")
      (Transformation|SetActorScale3D "0.100000,0.100000,0.100000")
      (Rendering|Material|SetMaterial _shipmesh 0 "/Game/Ships/SciFi_Fighter-MK6-OBJ/SciFi_Fighter_MK6Mat.SciFi_Fighter_MK6Mat")))
  (bind _output_get_2 (Variables|Default|SetspawnLocation spawnLoc))
  (bind _output_get_3 (Variables|Default|SetcurrLocation _output_get_2))
  (Transformation|SetActorLocation _output_get_3 false false)
  (Transformation|SetRelativeRotation _shipmesh (Variables|Default|GetdefaultRot) false false)
  (Variables|Default|SetforwardVector (Transformation|GetActorForwardVector))
  (Variables|Default|SetupVector (Transformation|GetActorUpVector)))

(fn Move
  (params (axisVal :type Float%20%28single-precision%29))
  (CallFunction|Accelerate axisVal)
  (Transformation|SetActorLocation (+ (Variables|Default|GetcurrLocation) (* (Variables|Default|GetforwardVector) (* (Variables|Default|GetcurrSpeed) (Variables|Default|GettimeSinceTick)))) false false)
  (Variables|Default|SetcurrLocation (+ (Variables|Default|GetcurrLocation) (* (Variables|Default|GetforwardVector) (* (Variables|Default|GetcurrSpeed) (Variables|Default|GettimeSinceTick))))))

(fn Accelerate
  (params (axisVal :type Float%20%28single-precision%29))
  (bind _accelrate (Variables|Default|GetaccelRate))
  (bind _maxspeed (Variables|Default|GetmaxSpeed))
  (if (> axisVal 0.0) ; Greater than 0? (Accel)
    (Variables|Default|SetcurrSpeed (Math|Float|Clamp(Float) (+ (Variables|Default|GetcurrSpeed) _accelrate) 0.0 _maxspeed))
    (elif (< axisVal 0.0) ; Less than 0? (Decel)
      (Variables|Default|SetcurrSpeed (Math|Float|Clamp(Float) (+ (Variables|Default|GetcurrSpeed) (* _accelrate -1.0)) 0.0 _maxspeed)))))

(fn Yaw
  (params (axisVal :type Float%20%28single-precision%29))
  (Transformation|AddActorLocalRotation (Math|Rotator|MakeRotator 0.0 0.0 axisVal) false false)
  (Variables|Default|SetforwardVector (Math|Vector|RotateVectorAroundAxis (Variables|Default|GetforwardVector) axisVal (Variables|Default|GetupVector))))

(fn Pitch
  (params (axisVal :type Float%20%28single-precision%29))
  (Transformation|AddActorLocalRotation (Math|Rotator|MakeRotator 0.0 axisVal 0.0) false false)
  (Variables|Default|SetforwardVector (Math|Vector|RotateVectorAroundAxis (Variables|Default|GetforwardVector) axisVal (Math|Vector|CrossProduct (Variables|Default|GetforwardVector) (Variables|Default|GetupVector))))
  (Variables|Default|SetupVector (Math|Vector|RotateVectorAroundAxis (Variables|Default|GetupVector) axisVal (Math|Vector|CrossProduct (Variables|Default|GetforwardVector) (Variables|Default|GetupVector)))))

(fn Roll
  (params (axisVal :type Float%20%28single-precision%29))
  (Transformation|AddActorLocalRotation (Math|Rotator|MakeRotator axisVal 0.0 0.0) false false)
  (Variables|Default|SetupVector (Math|Vector|RotateVectorAroundAxis (Variables|Default|GetupVector) axisVal (Variables|Default|GetforwardVector))))