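; Base game mode that hands the player's saved ship loadout to the pilot controller and spawns the player ship.
; On BeginPlay it copies component enums and the ship struct from the game instance into Pilot_ControllerBP.
; Weapons come from the controller's LoadWeapons for the hull, with the saved damage and fire-rate offsets merged per slot.
; It then spawns a PlayerBP at the origin and has the controller possess it.
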(event EventBeginPlay
  (bind _assfgame_instance_bp (Utilities|Casting|CastToSFGameInstanceBP (Game|GetGameInstance)))
  (bind _aspilot_controller_bp (Utilities|Casting|CastToPilot_ControllerBP (Game|GetPlayerController 0)))
  (Variables|/Game/Blueprints/Pilot_ControllerBP.Pilot_ControllerBP_C|SethullEnum _aspilot_controller_bp (Variables|/Game/Blueprints/SFGameInstanceBP.SFGameInstanceBP_C|GethullEnum _assfgame_instance_bp))
  (Variables|/Game/Blueprints/Pilot_ControllerBP.Pilot_ControllerBP_C|SetengineEnum _aspilot_controller_bp (Variables|/Game/Blueprints/SFGameInstanceBP.SFGameInstanceBP_C|GetengineEnum _assfgame_instance_bp))
  (Variables|/Game/Blueprints/Pilot_ControllerBP.Pilot_ControllerBP_C|SetshieldEnum _aspilot_controller_bp (Variables|/Game/Blueprints/SFGameInstanceBP.SFGameInstanceBP_C|GetshieldEnum _assfgame_instance_bp))
  (Variables|/Game/Blueprints/Pilot_ControllerBP.Pilot_ControllerBP_C|SetpowerEnum _aspilot_controller_bp (Variables|/Game/Blueprints/SFGameInstanceBP.SFGameInstanceBP_C|GetpowerEnum _assfgame_instance_bp))
  (Variables|/Game/Blueprints/Pilot_ControllerBP.Pilot_ControllerBP_C|SetweaponEnums _aspilot_controller_bp (Variables|/Game/Blueprints/SFGameInstanceBP.SFGameInstanceBP_C|Getweapons _assfgame_instance_bp))
  (bind _weapons (Default|LoadWeapons _aspilot_controller_bp (.hull (Utilities|Struct|BreakShipStruct (Variables|/Game/Blueprints/SFGameInstanceBP.SFGameInstanceBP_C|Getship _assfgame_instance_bp)))))
  (for (_array_element _array_index) (.weapons (Utilities|Struct|BreakShipStruct (Variables|/Game/Blueprints/SFGameInstanceBP.SFGameInstanceBP_C|Getship _assfgame_instance_bp)))
    (Utilities|Array|SetArrayElem _weapons _array_index (Utilities|Struct|MakeWeaponStruct (.relativeLocation (Utilities|Struct|BreakWeaponStruct (Utilities|Array|Get(acopy) _weapons _array_index))) (.damage (Utilities|Struct|BreakWeaponStruct (Utilities|Array|Get(acopy) _weapons _array_index))) (.fireRate (Utilities|Struct|BreakWeaponStruct (Utilities|Array|Get(acopy) _weapons _array_index))) (.fireCost (Utilities|Struct|BreakWeaponStruct (Utilities|Array|Get(acopy) _weapons _array_index))) (.laserSpeed (Utilities|Struct|BreakWeaponStruct (Utilities|Array|Get(acopy) _weapons _array_index))) (.laserColor (Utilities|Struct|BreakWeaponStruct (Utilities|Array|Get(acopy) _weapons _array_index))) (.energyCost (Utilities|Struct|BreakWeaponStruct (Utilities|Array|Get(acopy) _weapons _array_index))) (.damageOffset (Utilities|Struct|BreakWeaponStruct _array_element)) (.fireRateOffset (Utilities|Struct|BreakWeaponStruct _array_element)))))
  (Variables|/Game/Blueprints/Pilot_ControllerBP.Pilot_ControllerBP_C|Setship _aspilot_controller_bp (Utilities|Struct|MakeShipStruct (.hull (Utilities|Struct|BreakShipStruct (Variables|/Game/Blueprints/SFGameInstanceBP.SFGameInstanceBP_C|Getship _assfgame_instance_bp))) (.engine (Utilities|Struct|BreakShipStruct (Variables|/Game/Blueprints/SFGameInstanceBP.SFGameInstanceBP_C|Getship _assfgame_instance_bp))) (.shield (Utilities|Struct|BreakShipStruct (Variables|/Game/Blueprints/SFGameInstanceBP.SFGameInstanceBP_C|Getship _assfgame_instance_bp))) (.power (Utilities|Struct|BreakShipStruct (Variables|/Game/Blueprints/SFGameInstanceBP.SFGameInstanceBP_C|Getship _assfgame_instance_bp))) _weapons))
  (bind _returnvalue (Game|SpawnActorfromClass "/Game/Blueprints/PlayerBP.PlayerBP_C" (Math|Conversions|ToTransform(Vector) "0, 0, 0") "AlwaysSpawn" 0 0 0))
  (Pawn|Possess _aspilot_controller_bp _returnvalue))

(event EventTick
  (params (DeltaSeconds :type Float%20%28single-precision%29)))

(fn ConstructionScript)