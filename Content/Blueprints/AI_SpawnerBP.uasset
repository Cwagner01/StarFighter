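; AI spawner actor meant to create AI pilot agents over time, currently inactive because its spawn logic is disconnected from any event.
; The unwired logic caps total spawns, forces one after a maximum wait, and rolls a time-weighted random chance after a minimum wait.
; The Spawn function places a pilot slightly offset from the spawner, skipping it if colliding, and records it in Spawns.
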(event EventBeginPlay)

(event Collision|EventActorBeginOverlap
  (params (OtherActor :type Actor%20Object%20Reference)))

(event EventTick
  (params (DeltaSeconds :type Float%20%28single-precision%29)))

(fn ConstructionScript)

(fn Spawn
  (bind _returnvalue (Game|SpawnActorfromClass "/Game/Blueprints/AI_PilotBP.AI_PilotBP_C" (Math|Conversions|ToTransform(Vector) (+ (Transformation|GetActorLocation) (* (Variables|Default|GetForwardVector) 1e+01))) "DontSpawnIfColliding" 0 0))
  (Utilities|Array|Add (Variables|Default|Getspawns) _returnvalue))