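; Blueprint function library of miscellaneous helpers, holding a distance calculation between two points.
; DistanceTo takes Source and Target vectors and returns their straight-line 3D distance.
; It computes the Euclidean length by hand, taking the square root of the summed squared X, Y and Z differences.
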(fn Distanceto
  (params (source :type Vector) (target :type Vector))
  (bind (_x _y _z) (Math|Vector|BreakVector source))
  (bind (_x_2 _y_2 _z_2) (Math|Vector|BreakVector target))
  (return (Math|Float|Sqrt (+ (Math|Float|Square (- _x _x_2)) (Math|Float|Square (- _y _y_2)) (Math|Float|Square (- _z _z_2))))))