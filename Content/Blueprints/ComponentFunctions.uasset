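; Function library for reading and editing a ship's component loadout of hull, engine, shield, power and weapons.
; Setters rebuild the ship struct with one part swapped; the single-weapon setter writes into the weapons array by index, resizing to fit.
; Loaders fetch each component type from its data table, using the enum name as the row name.
; Convenience getters expose max speed, acceleration and turn rate from the engine.
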(fn SetEngine
  (params (ship :type Ship%20Struct%20Structure) (engine :type Engine%20Struct%20Structure))
  (bind (_hull _engine _shield _power _weapons) (Utilities|Struct|BreakShipStruct ship))
  (return (Utilities|Struct|MakeShipStruct _hull engine _shield _power _weapons)))

(fn SetHull
  (params (ship :type Ship%20Struct%20Structure) (hull :type Hull%20Struct%20Structure))
  (bind (_hull _engine _shield _power _weapons) (Utilities|Struct|BreakShipStruct ship))
  (return (Utilities|Struct|MakeShipStruct hull _engine _shield _power _weapons)))

(fn SetShield
  (params (ship :type Ship%20Struct%20Structure) (shield :type Shield%20Struct%20Structure))
  (bind (_hull _engine _shield _power _weapons) (Utilities|Struct|BreakShipStruct ship))
  (return (Utilities|Struct|MakeShipStruct _hull _engine shield _power _weapons)))

(fn SetPower
  (params (ship :type Ship%20Struct%20Structure) (power :type Power%20Struct%20Structure))
  (bind (_hull _engine _shield _power _weapons) (Utilities|Struct|BreakShipStruct ship))
  (return (Utilities|Struct|MakeShipStruct _hull _engine _shield power _weapons)))

(fn SetSingleWeapon
  (params (ship :type Ship%20Struct%20Structure) (newWeapon :type Weapon%20Struct%20Structure) (index :type Integer))
  (bind (_hull _engine _shield _power _weapons) (Utilities|Struct|BreakShipStruct ship))
  (Utilities|Array|SetArrayElem _weapons index newWeapon true)
  (return (Utilities|Struct|MakeShipStruct _hull _engine _shield _power _weapons)))

(fn SetWeapons
  (params (ship :type Ship%20Struct%20Structure) (weapons :type Array%20of%20Weapon%20Struct%20Structures))
  (bind (_hull _engine _shield _power) (Utilities|Struct|BreakShipStruct ship))
  (return (Utilities|Struct|MakeShipStruct _hull _engine _shield _power weapons)))

(fn GetEngine
  (params (ship :type Ship%20Struct%20Structure))
  (return (.engine (Utilities|Struct|BreakShipStruct ship))))

(fn GetHull
  (params (ship :type Ship%20Struct%20Structure))
  (return (.hull (Utilities|Struct|BreakShipStruct ship))))

(fn GetShield
  (params (ship :type Ship%20Struct%20Structure))
  (return (.shield (Utilities|Struct|BreakShipStruct ship))))

(fn GetPower
  (params (ship :type Ship%20Struct%20Structure))
  (return (.power (Utilities|Struct|BreakShipStruct ship))))

(fn GetSingleWeapon
  (params (ship :type Ship%20Struct%20Structure) (index :type Integer))
  (return (Utilities|Array|Get(acopy) (.weapons (Utilities|Struct|BreakShipStruct ship)) index)))

(fn GetWeapons
  (params (ship :type Ship%20Struct%20Structure))
  (return (.weapons (Utilities|Struct|BreakShipStruct ship))))

(fn LoadHull
  (params (hullEnum :type HullEnum%20Enum))
  (bind _returnvalue (Utilities|GetDataTableRow "/Game/Blueprints/Tables/HullTable.HullTable" (Utilities|String|StringToName (Utilities|String|EnumtoString hullEnum)))
    (:then
      (return _returnvalue))
    (:RowNotFound
      (return ""))))

(fn LoadWeapon
  (params (weaponEnum :type WeaponEnum%20Enum))
  (bind _returnvalue (Utilities|GetDataTableRow "/Game/Blueprints/Tables/WeaponTable.WeaponTable" (Utilities|String|StringToName (Utilities|String|EnumtoString weaponEnum)))
    (:then
      (return _returnvalue))
    (:RowNotFound
      (return ""))))

(fn LoadShield
  (params (shieldEnum :type ShieldEnum%20Enum))
  (bind _returnvalue (Utilities|GetDataTableRow "/Game/Blueprints/Tables/ShieldTable.ShieldTable" (Utilities|String|StringToName (Utilities|String|EnumtoString shieldEnum)))
    (:then
      (return _returnvalue))
    (:RowNotFound
      (return ""))))

(fn LoadPower
  (params (powerEnum :type PowerEnum%20Enum))
  (bind _returnvalue (Utilities|GetDataTableRow "/Game/Blueprints/Tables/PowerTable.PowerTable" (Utilities|String|StringToName (Utilities|String|EnumtoString powerEnum)))
    (:then
      (return _returnvalue))
    (:RowNotFound
      (return ""))))

(fn LoadEngine
  (params (engineEnum :type EngineEnum%20Enum))
  (bind _returnvalue (Utilities|GetDataTableRow "/Game/Blueprints/Tables/EngineTable.EngineTable" (Utilities|String|StringToName (Utilities|String|EnumtoString engineEnum)))
    (:then
      (return _returnvalue))
    (:RowNotFound
      (return ""))))

(fn GetMaxSpeed
  (params (ship :type Ship%20Struct%20Structure))
  (bind _engine (CallFunction|GetEngine ship))
  (return (.maxSpeed (Utilities|Struct|BreakEngineStruct _engine))))

(fn GetAccelRate
  (params (ship :type Ship%20Struct%20Structure))
  (bind _engine (CallFunction|GetEngine ship))
  (return (.accelRate (Utilities|Struct|BreakEngineStruct _engine))))

(fn GetTurnRate
  (params (ship :type Ship%20Struct%20Structure))
  (bind _engine (CallFunction|GetEngine ship))
  (return (.turnRate (Utilities|Struct|BreakEngineStruct _engine))))