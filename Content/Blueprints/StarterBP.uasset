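; StarterBP is a player-controlled flying craft with six-axis-style steering, twin projectile guns and health.
; Move input adjusts a clamped speed and translates the actor unswept along a manually tracked forward vector.
; Yaw, pitch and roll inputs apply local rotations while rotating stored forward and up vectors.
; Holding Fire spawns BP_Projectile from Left and Right on a looping timer; damage reduces health and destroys the actor at zero.
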(event Custom|FireReset
  ;[1 1 1] Fire
  (CallFunction|Fire (Variables|Default|GetLeft))
  (CallFunction|Fire (Variables|Default|GetRight)))

(event Game|Damage|EventAnyDamage
  (params (Damage :type Float%20%28single-precision%29) (DamageType :type Damage%20Type%20Object%20Reference) (InstigatedBy :type Controller%20Object%20Reference) (DamageCauser :type Actor%20Object%20Reference))
  (CallFunction|TakeDamage Damage))

(event EventTick
  (params (DeltaSeconds :type Float%20%28single-precision%29))
  (Variables|Default|SettimeSinceTick DeltaSeconds))

(event Input|ActionEvents|InputActionFire
  (params (Key :type Key%20Structure :default "AnyKey"))
  ;[1 1 1] Fire
  (:Pressed
    (bind _returnvalue (Utilities|Time|SetTimerbyFunctionName 0 "FireReset" 0.3 true))
    (Variables|Default|SettimeHandle _returnvalue)
    (CallFunction|Fire (Variables|Default|GetLeft))
    (CallFunction|Fire (Variables|Default|GetRight)))
  (:Released
    (Utilities|Time|ClearandInvalidateTimerbyHandle (Variables|Default|GettimeHandle))))

(event Input|AxisEvents|InputAxisYaw
  (params (AxisValue :type Float%20%28single-precision%29))
  ;[1 1 1] Yaw
  (Transformation|AddActorLocalRotation (Math|Rotator|MakeRotator 0.0 0.0 AxisValue) false false)
  (Variables|Default|SetforwardVector (Math|Vector|RotateVectorAroundAxis (Variables|Default|GetforwardVector) AxisValue (Variables|Default|GetupVector))))

(event Input|AxisEvents|InputAxisPitch
  (params (AxisValue :type Float%20%28single-precision%29))
  ;[1 1 1] Pitch
  (Transformation|AddActorLocalRotation (Math|Rotator|MakeRotator 0.0 AxisValue 0.0) false false)
  (Variables|Default|SetforwardVector (Math|Vector|RotateVectorAroundAxis (Variables|Default|GetforwardVector) AxisValue (Math|Vector|CrossProduct (Variables|Default|GetupVector) (Variables|Default|GetforwardVector))))
  (Variables|Default|SetupVector (Math|Vector|RotateVectorAroundAxis (Variables|Default|GetupVector) AxisValue (Math|Vector|CrossProduct (Variables|Default|GetupVector) (Variables|Default|GetforwardVector)))))

(event Input|AxisEvents|InputAxisRoll
  (params (AxisValue :type Float%20%28single-precision%29))
  ;[1 1 1] Roll
  (Transformation|AddActorLocalRotation (Math|Rotator|MakeRotator AxisValue 0.0 0.0) false false)
  (Variables|Default|SetupVector (Math|Vector|RotateVectorAroundAxis (Variables|Default|GetupVector) AxisValue (Variables|Default|GetforwardVector))))

(event Input|AxisEvents|InputAxisMove
  (params (AxisValue :type Float%20%28single-precision%29))
  ;[1 1 1] Move
  (CallFunction|Accelerate AxisValue)
  (Transformation|SetActorLocation (+ (Transformation|GetActorLocation) (* (Variables|Default|GetforwardVector) (* (Variables|Default|GetcurrSpeed) (Variables|Default|GettimeSinceTick)))) false false))

(fn ConstructionScript)

(fn Accelerate
  (params (AxisValue :type Float%20%28single-precision%29))
  (bind _accelfactor (Variables|Default|GetaccelFactor))
  (bind _maxspeed (Variables|Default|GetmaxSpeed))
  (if (> AxisValue 0.0) ; Greater than 0? (Accel)
    (bind _output_get (Variables|Default|SetcurrSpeed (Math|Float|Clamp(Float) (+ (Variables|Default|GetcurrSpeed) _accelfactor) 0.0 _maxspeed)))
    (elif (< AxisValue 0.0) ; Less than 0? (Decel)
      (bind _output_get_2 (Variables|Default|SetcurrSpeed (Math|Float|Clamp(Float) (+ (Variables|Default|GetcurrSpeed) (* _accelfactor -1.0)) 0.0 _maxspeed))))))

(fn Fire
  (params (Location :type Scene%20Component%20Object%20Reference))
  (Game|SpawnActorfromClass "/Game/Blueprints/BP_Projectile.BP_Projectile_C" (Transformation|GetWorldTransform Location) "AlwaysSpawn" 0 (Math|Color|MakeColor 0.2 0.3 1.0 1.0) 3.25e+03 self (Transformation|GetWorldLocation Location) (Variables|Default|GetforwardVector)))

(fn TakeDamage
  (params (damage :type Float%20%28single-precision%29))
  (Variables|Default|Sethealth (Math|Float|Clamp(Float) (- (Variables|Default|Gethealth) damage) 0.0 1e+02))
  (if (<= (Variables|Default|Gethealth) 0.0)
    (Actor|DestroyActor)))